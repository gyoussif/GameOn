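; Main menu player controller that switches input mode according to whether the mouse cursor should be shown.
; UpdateInputMode sets cursor visibility, then applies either Game and UI with a widget to focus, or Game Only with the mouse moved to the desktop resolution coordinates.
; An OnceBranch macro pairs two DoOnce nodes that reset each other, so each mode is applied only when the condition changes.
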(event Custom|UpdateInputMode
  (params (ShowMouseCursor :type Boolean) (InWidgetToFocus :type Widget%20Object%20Reference))
  (bind _self self)
  ;[0 0 0] Update Input Mode
  (bind _output_get (Variables|Default|SetbShowMouseCursor ShowMouseCursor))
  (Utilities|OnceBranch _output_get
    (:True
      (Input|SetInputModeGameandUI _self InWidgetToFocus "DoNotLock" true false))
    (:False
      (Input|SetInputModeGameOnly _self false)
      (bind _returnvalue (Settings|GetGameUserSettings))
      (Class|PlayerController|SetMouseLocation (.x (Class|GameUserSettings|GetDesktopResolution _returnvalue)) (.y (Class|GameUserSettings|GetDesktopResolution _returnvalue))))))

(fn ConstructionScript)